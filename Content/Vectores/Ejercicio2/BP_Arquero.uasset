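; BP_Arquero is an archer actor in a vector exercise that fires BP_Flecha arrows while attacking is enabled.
; A looping half-second timer started on BeginPlay checks the Ataque flag and spawns an arrow at the actor's location.
; Each arrow's velocity is VelocidadDeFlecha times MultiplicaciónVel, with setter functions for base velocity and attack flag.
; A long-lived debug box marks its position, and printed messages show its state.
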(event Custom|Disparar
  (Development|PrintString "Esperando")
  (if (Variables|Default|GetAtaque)
    (Development|PrintString "Disparajdo")
    (CallFunction|SpawnFlecha)))

(event EventBeginPlay
  (Utilities|Time|SetTimerbyEvent (delegate Custom|Disparar) 0.5 true)
  (Rendering|Debug|DrawDebugBox (Transformation|GetActorLocation) "50.000000,50.000000,50.000000" "(R=1.000000,G=0.312801,B=0.000000,A=1.000000)" "0, 0, 0" 3.6e+03 1e+01))

(fn ConstructionScript)

(fn SpawnFlecha
  (Game|SpawnActorfromClass "/Game/Vectores/Ejercicio1/BP_Flecha.BP_Flecha_C" (Math|Transform|MakeTransform (Transformation|GetActorLocation) "0, 0, 0" "1.000000,1.000000,1.000000") "Undefined" "MultiplyWithRoot" 0 (* (Variables|Default|GetVelocidad%20De%20Flecha) (Variables|Default|GetMultiplicaciónVel)) 0))

(fn SetVelocidadFlecha
  (params (Velocidad :type Vector))
  (Variables|Default|SetVelocidad%20De%20Flecha Velocidad))

(fn PuedoAtacar?
  (params (Ataque? :type Boolean))
  (Variables|Default|SetAtaque Ataque?))